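; Base enemy Character that takes bullet damage, dies and randomly drops pickups.
; Bullet overlaps subtract Health; Tick detects zero health, disables capsule collision, halts movement and starts a timer to Destroy.
; Destroy independently rolls for health and ammo drops, then removes the actor and any DesertPatrol weapon.
; While alive, Tick fakes gravity with LaunchCharacter; DecreaseHealth can set IsDead directly, bypassing that death sequence.
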(event EventBeginPlay)

(event Collision|EventActorBeginOverlap
  (params (OtherActor :type Actor%20Object%20Reference))
  (bind _asbullet_bp (Utilities|Casting|CastToBullet_BP OtherActor))
  (Variables|Default|SetHealth (- (Variables|Default|GetHealth) (Math|Float|Truncate (Variables|/Game/Guns/Blueprints/Bullet_BP.Bullet_BP_C|GetDamage _asbullet_bp)))))

(event EventTick
  (params (DeltaSeconds :type Float%20%28single-precision%29))
  (if (Variables|Default|GetIsDead)
    _
    (else
      (CallFunction|SimGravity DeltaSeconds)))
  (if (and (not (Variables|Default|GetIsDead)) (<= (Variables|Default|GetHealth) 0))
    (Variables|Default|SetIsDead true)
    (Utilities|Time|SetTimerbyFunctionName 0 "Destroy" 3.0)
    (Collision|SetCollisionEnabled (Variables|Collision|GetCapsuleComponent) "NoCollision")
    (Character|LaunchCharacter "0, 0, 0" true true)))

(fn ConstructionScript)

(fn DecreaseHealth
  (params (Amount :type Integer))
  (Development|PrintString "hit")
  (Math|Integer|CompareInt Amount (Variables|Default|GetHealth)
    (:>
      (Variables|Default|SetIsDead true :!label _label))
    (:==
      (goto _label))
    (:<
      (Variables|Default|SetHealth (- (Variables|Default|GetHealth) Amount)))))

(fn Reset)

(fn Destroy
  (bind _returnvalue (Transformation|GetActorLocation))
  (Math|Integer|CompareInt (Math|Random|RandomInteger 10) 3
    (:>
      _)
    (:==
      (Game|SpawnActorfromClass "/Game/Blueprints/HealthPack.HealthPack_C" (Math|Transform|MakeTransform _returnvalue "0, 0, 0" "1,1,1") "Undefined" 0 0 :!label _label))
    (:<
      (goto _label)))
  (Math|Integer|CompareInt (Math|Random|RandomInteger 10) 5
    (:>
      _)
    (:==
      (Game|SpawnActorfromClass "/Game/Guns/Blueprints/AmmBox_BP.AmmBox_BP_C" (Math|Transform|MakeTransform _returnvalue "0, 0, 0" "1,1,1") "Undefined" 0 0 :!label _label_2))
    (:<
      (goto _label_2)))
  (bind _asdesert_patrol_bp (Utilities|Casting|CastToDesertPatrol_BP self)
    (:then
      (Actor|DestroyActor (Variables|/Game/Enemies/Blueprints/DesertPatrol_BP.DesertPatrol_BP_C|GetWeapon _asdesert_patrol_bp)))
    (:CastFailed
      _))
  (Actor|DestroyActor))

(fn SimGravity
  (params (DeltaSeconds :type Float%20%28single-precision%29))
  (if (not (.bwalkablefloor (Pawn|Components|CharacterMovement|FindFloor (Variables|Character|GetCharacterMovement) (Transformation|GetActorLocation))))
    (Character|LaunchCharacter (Math|Vector|MakeVector 0.0 0.0 (* (Components|Movement|GetGravityZ (Variables|Character|GetCharacterMovement)) DeltaSeconds)) false false)))