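; Enemy spawn point that creates one enemy at its own location when SpawnEnemy is called.
; EnemyToSpawn selects a Desert Patrol or Brute, each with its own particle effect, then the spawn gets a default controller.
; IsEnemyDead reports true whenever the stored enemy reference is invalid or the encounter has not started.
; The event graph is empty, so spawning relies on external calls.
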(event EventBeginPlay)

(event Collision|EventActorBeginOverlap
  (params (OtherActor :type Actor%20Object%20Reference)))

(event EventTick
  (params (DeltaSeconds :type Float%20%28single-precision%29)))

(fn ConstructionScript)

(fn SpawnEnemy
  (bind _returnvalue (Transformation|GetActorLocation))
  (bind _returnvalue_2 (Math|Conversions|ToTransform(Vector) _returnvalue))
  (Variables|Default|SetEncounterStarted true)
  (switch int (Variables|Default|GetEnemy%20To%20Spawn)
    (:0
      (bind _returnvalue_3 (Game|SpawnActorfromClass "/Game/Enemies/Blueprints/DesertPatrol_BP.DesertPatrol_BP_C" _returnvalue_2 "Undefined" 0 0))
      (bind _output_get (Variables|Default|SetEnemyObject _returnvalue_3))
      (Effects|SpawnEmitteratLocation "/Game/Realistic_Starter_VFX_Pack_Vol2/Particles/Destruction/P_Destruction_Electric.P_Destruction_Electric" _returnvalue)
      (Pawn|SpawnDefaultController _output_get))
    (:1
      (bind _returnvalue_4 (Game|SpawnActorfromClass "/Game/Enemies/Blueprints/Brute_BP.Brute_BP_C" _returnvalue_2 "Undefined" 0 0))
      (bind _output_get_2 (Variables|Default|SetEnemyObject _returnvalue_4))
      (Effects|SpawnEmitteratLocation "/Game/FXVarietyPack/Particles/P_ky_lightning2.P_ky_lightning2" _returnvalue)
      (Pawn|SpawnDefaultController _output_get_2))))

(fn IsEnemyDead
  (return (not (and (Variables|Default|GetEncounterStarted) (Utilities|IsValid (Variables|Default|GetEnemyObject))))))