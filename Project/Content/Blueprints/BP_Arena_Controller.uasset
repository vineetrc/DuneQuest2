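; Arena encounter controller that runs wave-based enemy spawning across five zones once the player enters its trigger.
; Overlap by a BP_Player_MovementBase pawn starts the encounter once, after which Tick calls AttemptZoneSpawn for every zone.
; Each zone with spawns remaining checks whether all its spawners' enemies are dead, then respawns them and decrements that zone's count.
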(event OnComponentBeginOverlap(EncounterTrigger)
  (params (OverlappedComponent :type Primitive%20Component%20Object%20Reference) (OtherActor :type Actor%20Object%20Reference) (OtherComp :type Primitive%20Component%20Object%20Reference) (OtherBodyIndex :type Integer) (bFromSweep :type Boolean) (SweepResult :type Hit%20Result%20Structure%20%28by%20ref%29))
  (Utilities|Casting|CastToBP_Player_MovementBase OtherActor)
  (if (not (Variables|Default|GetIsEncounterStarted))
    (Variables|Default|SetIsEncounterStarted true)
    (for _index (range 0 4)
      (CallFunction|AttemptZoneSpawn _index))))

(event EventBeginPlay)

(event Collision|EventActorBeginOverlap
  (params (OtherActor :type Actor%20Object%20Reference)))

(event EventTick
  (params (DeltaSeconds :type Float%20%28single-precision%29))
  (if (Variables|Default|GetIsEncounterStarted)
    (for _index (range 0 4)
      (CallFunction|AttemptZoneSpawn _index))))

(fn ConstructionScript)

(fn StartEncounter
  (Variables|Default|SetIsEncounterStarted true)
  (for _index (range 0 4)
    (CallFunction|AttemptZoneSpawn _index)))

(fn AttemptZoneSpawn
  (params (ZoneNumber :type Integer))
  (switch int ZoneNumber
    (:0
      (Math|Integer|CompareInt (Variables|Default|GetZone0SpawnAmount)
        (:>
          (LocalVariables|SetCurrentZone (Variables|Default|GetZone0)))))
    (:1
      (Math|Integer|CompareInt (Variables|Default|GetZone1SpawnAmount)
        (:>
          (LocalVariables|SetCurrentZone (Variables|Default|GetZone1)))))
    (:2
      (Math|Integer|CompareInt (Variables|Default|GetZone2SpawnAmount)
        (:>
          (LocalVariables|SetCurrentZone (Variables|Default|GetZone2)))))
    (:3
      (Math|Integer|CompareInt (Variables|Default|GetZone3SpawnAmount)
        (:>
          (LocalVariables|SetCurrentZone (Variables|Default|GetZone3)))))
    (:4
      (Math|Integer|CompareInt (Variables|Default|GetZone4SpawnAmount)
        (:>
          (LocalVariables|SetCurrentZone (Variables|Default|GetZone4))))))
  (for _array_element (LocalVariables|GetCurrentZone)
    (bind _isdead (Default|IsEnemyDead _array_element))
    (LocalVariables|SetAllDead (and _isdead (LocalVariables|GetAllDead))))
  (if (LocalVariables|GetAllDead)
    (for _array_element_2 (LocalVariables|GetCurrentZone)
      (Default|SpawnEnemy _array_element_2))
    (switch int ZoneNumber
      (:0
        (Math|Integer|DecrementInt (Variables|Default|GetZone0SpawnAmount)))
      (:1
        (Math|Integer|DecrementInt (Variables|Default|GetZone1SpawnAmount)))
      (:2
        (Math|Integer|DecrementInt (Variables|Default|GetZone2SpawnAmount)))
      (:3
        (Math|Integer|DecrementInt (Variables|Default|GetZone3SpawnAmount)))
      (:4
        (Math|Integer|DecrementInt (Variables|Default|GetZone4SpawnAmount))))))