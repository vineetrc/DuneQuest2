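; Player character Blueprint that adds the HUD widget and handles health, hurt feedback, knockback and death.
; AnyDamage outside dash invincibility shows a hurt widget, subtracts health if the causer is valid, and launches the player horizontally away on heavy hits.
; Tick overrides velocity while KnockbackActive, though this file only ever clears that flag.
; Death adds a game-over widget, then immediately restores health, teleports to spawn and removes it; P applies self-damage.
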(event EventBeginPlay
  (|CallParentFunction)
  (bind _returnvalue (UserInterface|CreateWidget "/Game/Blueprints/HUD.HUD_C"))
  (UserInterface|Viewport|AddtoViewport _returnvalue 0)
  (Variables|Default|SetSpawn%20Location (Transformation|GetActorLocation)))

(event EventTick
  (params (DeltaSeconds :type Float%20%28single-precision%29))
  (bind _charactermovement (Variables|Character|GetCharacterMovement))
  (bind _knockbackvelocity (Variables|Default|GetKnockbackVelocity))
  (|CallParentFunction DeltaSeconds)
  (if (Variables|Default|GetKnockbackActive)
    (Class|PawnMovementComponent|ConsumeInputVector _charactermovement)
    (Variables|/Script/Engine.MovementComponent|SetVelocity _charactermovement (Math|Vector|MakeVector (.x _knockbackvelocity) (.y _knockbackvelocity) 0.0))))

(event Game|Damage|EventAnyDamage
  (params (Damage :type Float%20%28single-precision%29) (DamageType :type Damage%20Type%20Object%20Reference) (InstigatedBy :type Controller%20Object%20Reference) (DamageCauser :type Actor%20Object%20Reference))
  (bind _returnvalue (Transformation|GetActorLocation))
  (bind _returnvalue_2 (Transformation|GetActorLocation DamageCauser))
  (bind _returnvalue_3 (- _returnvalue _returnvalue_2))
  (bind _returnvalue_4 (Math|Vector2D|Normalize2D (Math|Vector2D|MakeVector2D (.x _returnvalue_3) (.y _returnvalue_3))))
  (bind _returnvalue_5 (* _returnvalue_4 1e+03))
  (if (not (Variables|Default|GetDashInvincibility))
    (Utilities|IsValid DamageCauser
      (:Is%20Valid
        (Variables|Default|SetHealth (- (Variables|Default|GetHealth) Damage))
        (if (> Damage 15.0)
          (Variables|Default|SetKnockbackActive false)
          (Variables|Default|SetKnockbackVelocity (Math|Vector2D|MakeVector2D (.x _returnvalue_5) (.y _returnvalue_5)))
          (Character|LaunchCharacter (Math|Vector|MakeVector (.x _returnvalue_5) (.y _returnvalue_5) 0.0) true true)))
      (:Is%20Not%20Valid
        _))
    (bind _returnvalue_6 (UserInterface|CreateWidget "/Game/Blueprints/HurtWidget.HurtWidget_C"))
    (UserInterface|Viewport|AddtoViewport _returnvalue_6 0)
    (if (<= (Variables|Default|GetHealth) 0.0)
      (bind _returnvalue_7 (UserInterface|CreateWidget "/Game/Blueprints/GameOver.GameOver_C"))
      (Variables|Default|SetGameOverWid _returnvalue_7)
      (UserInterface|Viewport|AddtoViewport _returnvalue_7 0)
      (Variables|Default|SetKnockbackActive false)
      (CallFunction|ResetGame)
      (else
        (Utilities|FlowControl|RetriggerableDelay 0.5)
        (Variables|Default|SetKnockbackActive false)))))

(event Input|KeyboardEvents|P
  (params (Key :type Key%20Structure :default "None"))
  (:Pressed
    (Game|Damage|ApplyDamage self 1e+01 0 0 "/Script/Engine.DamageType")))

(fn ConstructionScript
  (|CallParentFunction))

(fn ResetGame
  (Variables|Default|SetHealth 1e+02)
  (Transformation|SetActorLocation (Variables|Default|GetSpawn%20Location) false true)
  (Widget|RemovefromParent (Variables|Default|GetGameOverWid)))