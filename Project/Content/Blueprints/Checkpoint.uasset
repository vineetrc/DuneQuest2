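; Checkpoint actor that updates the player's spawn location when touched.
; A sphere overlap casts the other actor to BP_Player_HUD, stores the checkpoint's location as its SpawnLocation, plays a 2D sound and destroys the checkpoint, making it single-use.
; Each tick, its TextRender rotates to face the player pawn.
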(event OnComponentBeginOverlap(Sphere)
  (params (OverlappedComponent :type Primitive%20Component%20Object%20Reference) (OtherActor :type Actor%20Object%20Reference) (OtherComp :type Primitive%20Component%20Object%20Reference) (OtherBodyIndex :type Integer) (bFromSweep :type Boolean) (SweepResult :type Hit%20Result%20Structure%20%28by%20ref%29))
  (bind _asbp_player_hud (Utilities|Casting|CastToBP_Player_HUD OtherActor))
  (Variables|/Game/Blueprints/BP_Player_HUD.BP_Player_HUD_C|SetSpawn%20Location _asbp_player_hud (Transformation|GetActorLocation))
  (Audio|PlaySound2D "/Game/Sounds/checkpoint.checkpoint" 1.0 1.0 0.0 0 0)
  (Actor|DestroyActor))

(event EventBeginPlay)

(event Collision|EventActorBeginOverlap
  (params (OtherActor :type Actor%20Object%20Reference)))

(event EventTick
  (params (DeltaSeconds :type Float%20%28single-precision%29))
  (bind _textrender (Variables|Default|GetTextRender))
  (Transformation|SetRelativeRotation _textrender (Math|Rotator|FindLookatRotation (Transformation|GetWorldLocation _textrender) (Transformation|GetActorLocation (Game|Player|GetPlayerPawn 0))) false false))

(fn ConstructionScript)