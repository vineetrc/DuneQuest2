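; Player Blueprint that gives the character a primary gun with fire and reload input.
; On BeginPlay it spawns an AR weapon and attaches it to the gun socket on the Arms component.
; The Fire action calls the weapon's Fire, followed by an ammo check that leads nowhere.
; R reloads when ammo is below max, using DoOnce and a reload-time Delay to block repeats while IsReloading is set.
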(event EventBeginPlay
  (|CallParentFunction)
  (bind _returnvalue (Game|SpawnActorfromClass "/Game/Guns/Blueprints/AR_Weapon_BP.AR_Weapon_BP_C" (Math|Transform|MakeTransform "0.000000, 0, 0" "0, 0, 0" "1,1,1") "Undefined" 0 0))
  (bind _output_get (Variables|Default|SetPrimaryWeapon _returnvalue))
  (Transformation|AttachComponentToComponent _output_get (Variables|Default|GetArms) "gun_socket" "KeepRelative" "KeepRelative" "KeepRelative" true))

(event Input|ActionEvents|InputActionFire
  (params (Key :type Key%20Structure :default "None"))
  (bind _primaryweapon (Variables|Default|GetPrimaryWeapon))
  (:Pressed
    (Default|Fire _primaryweapon)
    (if (> (Variables|/Game/Guns/Blueprints/Weapon_bp.Weapon_BP_C|GetCurAmmo _primaryweapon) 0)
      _)))

(event Input|KeyboardEvents|R
  (params (Key :type Key%20Structure :default "None"))
  (bind _primaryweapon (Variables|Default|GetPrimaryWeapon))
  (bind _primaryweapon_2 (Variables|Default|GetPrimaryWeapon))
  (:Pressed
    (if (< (Variables|/Game/Guns/Blueprints/Weapon_bp.Weapon_BP_C|GetCurAmmo _primaryweapon) (Variables|/Game/Guns/Blueprints/Weapon_bp.Weapon_BP_C|GetMaxAmmo _primaryweapon))
      (Utilities|FlowControl|DoOnce false :!label _label
        (:Completed
          (Variables|Default|SetIsReloading true)
          (Default|Reload _primaryweapon_2)
          (Utilities|FlowControl|Delay (Variables|/Game/Guns/Blueprints/Weapon_bp.Weapon_BP_C|GetReloadTime _primaryweapon_2))
          (Variables|Default|SetIsReloading false)
          (goto _label Reset))))))

(fn ConstructionScript
  (|CallParentFunction))