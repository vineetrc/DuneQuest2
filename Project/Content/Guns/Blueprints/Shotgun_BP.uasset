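; Player shotgun built on a parent gun class, with its own ammo, spread and reload settings.
; Fire spends one round and loops ten randomly spread camera traces, spawning decals at impact points and bullet actors from the muzzle.
; A randomized muzzle flash and delayed load sound follow; empty or mid-reload shots dry-fire.
; Reload plays an animation, then after a delay refills from the player's AmmoCount.
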(event EventBeginPlay)

(event Collision|EventActorBeginOverlap
  (params (OtherActor :type Actor%20Object%20Reference)))

(event EventFire
  (if (and (> (Variables|Default|GetCurAmmo) 0) (not (Variables|/Game/Blueprints/BP_Player_Guns.BP_Player_Guns_C|GetIsReloading (.AsBP%20Player%20Guns (Utilities|Casting|CastToBP_Player_Guns (Game|GetPlayerCharacter 0))))))
    (CallFunction|CheckAmmo)
    (for _index (range 0 9)
      (bind (_muzzlepoint _impactpoint) (CallFunction|LineTrace))
      (CallFunction|SpawnDecalBullet _muzzlepoint _impactpoint _impactpoint))
    (Utilities|FlowControl|Sequence
      (:then_0
        (Utilities|MuzzleFlash))
      (:then_1
        (Utilities|FlowControl|Delay 0.5)
        (Audio|PlaySound2D "/Game/Guns/Sounds/Reload_Load.Reload_Load" 1.0 1.0 0.0 0 0)))
    (else
      (Audio|PlaySound2D "/Game/Guns/Sounds/DryFire.DryFire" 1.0 1.0 0.0 0 0))))

(event EventReload
  (Components|Animation|PlayAnimation (Variables|Default|GetWeapon) "/Game/Guns/Animations/MP5_Reload_anim.MP5_Reload_anim" false)
  (Utilities|FlowControl|Delay (Variables|Default|GetReloadTime))
  (bind _asbp_player_hud (Utilities|Casting|CastToBP_Player_HUD (Game|GetPlayerCharacter 0)))
  (Variables|Default|SetCurAmmo (Math|Integer|Min(Integer) (Variables|Default|GetMaxAmmo) (Variables|/Game/Blueprints/BP_Player_HUD.BP_Player_HUD_C|GetAmmo_Count _asbp_player_hud)))
  (Variables|/Game/Blueprints/BP_Player_HUD.BP_Player_HUD_C|SetAmmo_Count _asbp_player_hud (- (Variables|/Game/Blueprints/BP_Player_HUD.BP_Player_HUD_C|GetAmmo_Count _asbp_player_hud) (Math|Integer|Min(Integer) (Variables|Default|GetMaxAmmo) (Variables|/Game/Blueprints/BP_Player_HUD.BP_Player_HUD_C|GetAmmo_Count _asbp_player_hud))))
  (Development|PrintString "Hello"))

(event EventTick
  (params (DeltaSeconds :type Float%20%28single-precision%29))
  (|CallParentFunction DeltaSeconds)
  (Math|Integer|DecrementInt (Variables|Default|GetFireRate)))

(fn ConstructionScript
  (|CallParentFunction)
  (Variables|Default|SetMaxAmmo 7)
  (Variables|Default|SetCurAmmo 7)
  (Variables|Default|SetReloadTime 1.0)
  (Variables|Default|SetBulletSpray 3e+03))

(fn CheckAmmo
  (bind _returnvalue (Math|Random|RandomFloatinRange 0.7 1.2))
  (Math|Integer|DecrementInt (Variables|Default|GetCurAmmo)
    (:%20%20
      (if (not (Variables|/Game/Blueprints/BP_Player_Guns.BP_Player_Guns_C|GetIsReloading (.AsBP%20Player%20Guns (Utilities|Casting|CastToBP_Player_Guns (Game|GetPlayerCharacter 0)))))
        (Audio|PlaySound2D "/Game/Guns/Sounds/Shotgun_Blast.Shotgun_Blast" (+ _returnvalue 2.5) _returnvalue 0.0 0 0)
        (Components|Animation|PlayAnimation (Variables|Default|GetWeapon) "/Game/Guns/Animations/AK_Fire_anim.AK_Fire_anim" false)
        (Development|PrintString (Utilities|String|ToString(Integer) (Variables|Default|GetCurAmmo)))))))

(fn LineTrace
  (bind _returnvalue (Game|GetPlayerCharacter 0))
  (bind _bulletspray (Variables|Default|GetBulletSpray))
  (bind _muzzle (Variables|Default|GetMuzzle))
  (bind _returnvalue_2 (Transformation|GetWorldLocation _muzzle))
  (bind _returnvalue_3 (* _bulletspray -1.0))
  (bind _asbp_player_movement_base (Utilities|Casting|CastToBP_Player_MovementBase _returnvalue))
  (bind _camera (Variables|/Game/Blueprints/BP_Player_MovementBase.BP_Player_MovementBase_C|GetCamera _asbp_player_movement_base))
  (bind _returnvalue_4 (Transformation|GetWorldLocation _camera))
  (bind _outhit (Collision|LineTraceByChannel _returnvalue_4 (+ (+ (* (Math|Vector|GetForwardVector _camera) 2e+04) _returnvalue_4) (Math|Vector|MakeVector (Math|Random|RandomFloatinRange _returnvalue_3 _bulletspray) (Math|Random|RandomFloatinRange _returnvalue_3 _bulletspray) (Math|Random|RandomFloatinRange _returnvalue_3 _bulletspray))) "TraceTypeQuery1" false 0 "None")) ; Camera shot
  (Collision|LineTraceByChannel _returnvalue_2 (.ImpactPoint (Collision|BreakHitResult _outhit)) "TraceTypeQuery1" false 0 "None" true "(R=0.152520,G=1.000000,B=0.292612,A=1.000000)") ; Gunshot
  (return _returnvalue_2 (.ImpactPoint (Collision|BreakHitResult _outhit))))

(fn SpawnDecalBullet
  (params (Location :type Vector) (SpawnTransformPoint :type Vector) (ImpactPoint :type Vector))
  (Game|SpawnActorfromClass "/Game/Guns/Blueprints/BulletDecal_BP.BulletDecal_BP_C" (Math|Transform|MakeTransform SpawnTransformPoint (Math|Conversions|RotationFromXVector ImpactPoint) "0.025000,0.025000,0.025000") "Undefined" 0 0)
  (if (>= (Math|Random|RandomIntegerinRange 1 10) 1)
    (Game|SpawnActorfromClass "/Game/Guns/Blueprints/Bullet_BP.Bullet_BP_C" (Math|Transform|MakeTransform Location (Transformation|GetWorldRotation (Variables|/Game/Blueprints/BP_Player_MovementBase.BP_Player_MovementBase_C|GetCamera (.AsBP%20Player%20Movement%20Base (Utilities|Casting|CastToBP_Player_MovementBase (Game|GetPlayerCharacter 0))))) "0.050000,0.050000,0.050000") "Undefined" 0 0))
  (return))