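; Weapon Blueprint that works either as a carried gun or as a spinning world pickup, switched by IsOnPerson.
; When carried, it disables HitBox collision on BeginPlay; otherwise Tick yaws it at RotateSpeed, scaled by delta time.
; Overlapping the HitBox with a BP_Player_MovementBase destroys the actor, with no weapon grant in this graph.
; Fire and Reload are empty events here.
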(event OnComponentBeginOverlap(HitBox)
  (params (OverlappedComponent :type Primitive%20Component%20Object%20Reference) (OtherActor :type Actor%20Object%20Reference) (OtherComp :type Primitive%20Component%20Object%20Reference) (OtherBodyIndex :type Integer) (bFromSweep :type Boolean) (SweepResult :type Hit%20Result%20Structure%20%28by%20ref%29))
  (Utilities|Casting|CastToBP_Player_MovementBase OtherActor)
  (Actor|DestroyActor))

(event Custom|Fire)

(event Custom|Reload)

(event EventBeginPlay
  (if (Variables|Default|GetIsOnPerson)
    (Collision|SetCollisionEnabled (Variables|Default|GetHitBox) "NoCollision")))

(event EventTick
  (params (DeltaSeconds :type Float%20%28single-precision%29))
  (bind _returnvalue (Transformation|GetActorRotation))
  (if (not (Variables|Default|GetIsOnPerson))
    (Transformation|SetActorRotation (Math|Rotator|MakeRotator (.roll _returnvalue) (.pitch _returnvalue) (+ (* DeltaSeconds (Variables|Default|GetRotateSpeed)) (.yaw _returnvalue))))))

(fn ConstructionScript)